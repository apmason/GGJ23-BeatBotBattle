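; BP_Enemy is an enemy that walks toward a target location and dies when hit by a grabbable small cube.
; On BeginPlay, its movement component starts the walk while the mesh loops a rifle walk animation and an attached footstep sound plays.
; The first cube hit sets a dead flag, stops movement, plays a death animation and, if the footstep sound is valid, swaps it for a scream.
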(event `self.ReceiveBeginPlay`
  (`/Game/Blueprints/BP_EnemyMovementComponent.Start Walking` (`self.BP_EnemyMovementComponent`) 2.0 (`self.Target Location`))
  (`SkeletalMeshComponent.PlayAnimation` (`self.Mesh`) "/Game/Worker_Robot/Epic_Animations/Walk_Fwd_Rifle_Ironsights.Walk_Fwd_Rifle_Ironsights" true)
  (bind _returnvalue (`GameplayStatics.SpawnSoundAttached` "/Game/Audio/lumberjack-footsteps01.lumberjack-footsteps01" (`self.Mesh`) "None" (0.0 0.0 0.0) (struct) "KeepRelativeOffset" false 1.0 1.0 0.0 null null))
  (set `self.Walking Sound` _returnvalue))

(event `self.ReceiveHit`
  (params (MyComp :type "PrimitiveComponent Object Reference") (Other :type "Actor Object Reference") (OtherComp :type "PrimitiveComponent Object Reference") (bSelfMoved :type Boolean) (HitLocation :type "Vector Structure") (HitNormal :type "Vector Structure") (NormalImpulse :type "Vector Structure") (Hit :type "HitResult Structure (by ref)"))
  (cast `/Game/VRTemplate/Blueprints/Grabbable_SmallCube` Other)
  (`KismetSystemLibrary.PrintString` "HIT IN ACTOR" true true (struct :`G` 0.66 :`B` 1.0 :`A` 1.0) 30.0)
  (if (not (`self.Is Dead`))
    (set `self.Is Dead` true)
    (`/Game/Blueprints/BP_EnemyMovementComponent.Stop Walking` (`self.BP_EnemyMovementComponent`))
    (`SkeletalMeshComponent.PlayAnimation` (`self.Mesh`) "/Game/Worker_Robot/Epic_Animations/Death_1.Death_1" false)
    (`/Engine/EditorBlueprintResources/StandardMacros.IsValid` (`self.Walking Sound`)
      (:`Is Valid`
        (`AudioComponent.Stop` (`self.Walking Sound`))
        (set `self.Walking Sound` null)
        (`GameplayStatics.SpawnSoundAttached` "/Game/Audio/scream02.scream02" (`self.Mesh`) "None" (0.0 0.0 0.0) (struct) "KeepRelativeOffset" false 1.0 1.0 0.0 null null)))))

(fn `UserConstructionScript`)