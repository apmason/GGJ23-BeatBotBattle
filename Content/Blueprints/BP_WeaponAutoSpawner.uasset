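; Auto-respawning pickup point that keeps supplying grabbable beetroot weapons at the spawner's location.
; It spawns a Grabbable_BeetRoot on BeginPlay and binds to its grab component's OnGrabbed event.
; When grabbed, it unbinds, clears the reference and spawns a replacement after a short delay.
; Reset spawns a new one only if no valid grab component is currently tracked.
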(event `self.ReceiveBeginPlay`
  (`self.Spawn New Weapon`))

(event `Spawn New Weapon`
  (bind (_returnvalue_location _returnvalue_rotation) (`KismetMathLibrary.BreakTransform` (`self.GetTransform`)))
  (bind _returnvalue (`|SpawnActorFromClass` "/Game/VRTemplate/Blueprints/Grabbable_BeetRoot.Grabbable_BeetRoot_C" (`KismetMathLibrary.MakeTransform` _returnvalue_location _returnvalue_rotation (1.0 1.0 1.0)) "Undefined" "OverrideRootScale" null null))
  (bind _output_get (set `self.Grab Component` (`/Game/VRTemplate/Blueprints/Grabbable_BeetRoot.GrabComponent` _returnvalue)))
  (add `/Game/VRTemplate/Blueprints/GrabComponent.OnGrabbed` _output_get (delegate `Handle On Grab`)))

(event `Handle On Grab`
  (remove `/Game/VRTemplate/Blueprints/GrabComponent.OnGrabbed` (`self.Grab Component`) (delegate `Handle On Grab`))
  (set `self.Grab Component` null)
  (`KismetSystemLibrary.Delay` 3.0)
  (`self.Spawn New Weapon`))

(event `Reset`
  (`/Engine/EditorBlueprintResources/StandardMacros.IsValid` (`self.Grab Component`)
    (:`Is Not Valid`
      (`self.Spawn New Weapon`))))

(fn `UserConstructionScript`)