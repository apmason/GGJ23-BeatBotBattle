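; BP_Stage is a stage actor that spawns a set of enemies and signals completion once all of them are dead.
; Setup clears earlier enemies, then spawns BP_Enemy at each configured spawn location, but only when RandomizeSpawnPoints is off.
; Each enemy's death event triggers a recount of living enemies, firing StageCompleted at zero.
; The randomized branch is empty, and the check matching enemy count to spawn locations is disconnected.
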(event `Setup`
  (`self.Teardown`)
  (if (not (`self.Randomize Spawn Points`))
    (for _index (range (`self.NumEnemies`))
      (`KismetSystemLibrary.PrintString` (`KismetStringLibrary.Conv_IntToString` _index))
      (bind (_output_location _output_rotation) (`KismetMathLibrary.BreakTransform` (`|GetArrayItem` (`self.Spawn Locations`) _index)))
      (bind _returnvalue (`|SpawnActorFromClass` "/Game/Blueprints/BP_Enemy.BP_Enemy_C" (`KismetMathLibrary.MakeTransform` _output_location _output_rotation) "AdjustIfPossibleButAlwaysSpawn" "OverrideRootScale" self (0.0 0.0 0.0) null))
      (add `/Game/Blueprints/BP_Enemy.Enemy Died` _returnvalue (delegate `Handle Enemy Died`))
      (`KismetArrayLibrary.Array_Add` (`self.Enemies`) _returnvalue))))

(event `Handle Enemy Died`
  (if (== (`self.Get Num Enemies Remaining`) 0)
    (`self.Stage Completed` self)))

(event `Teardown`
  (for _array_element (`self.Enemies`)
    (`/Engine/EditorBlueprintResources/StandardMacros.IsValid` _array_element
      (:`Is Valid`
        (`self.K2_DestroyActor` _array_element))))
  (`KismetArrayLibrary.Array_Clear` (`self.Enemies`)))

(fn `Get Num Enemies Remaining`
  (returns (Remaining :type Integer))
  (locals (`Num Remaining` :type Integer))
  (set `local.Num Remaining` 0)
  (for _array_element (`self.Enemies`)
    (if (not (`/Game/Blueprints/BP_Enemy.Is Dead` _array_element))
      (set `local.Num Remaining` (+ (`local.Num Remaining`) 1))))
  (return (`local.Num Remaining`)))

(fn `UserConstructionScript`)