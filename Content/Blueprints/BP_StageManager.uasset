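; Stage manager that announces a numbered level on the HUD, then spawns and runs the active combat stage.
; SetHUD starts the flow: the level title shows for a short delay, then a BP_Stage spawns with a fixed enemy count and two gate spawn points.
; Restart resets the weapon spawner and rebuilds the current stage through Teardown and Setup.
; Stage completion is bound but its handler is empty, so levels do not advance.
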(event `Set HUD`
  (params (HUD :type "/Game/Widgets/WBP_HUD Object Reference"))
  (set `self.HUD` HUD)
  (set `self.Current Stage` 0)
  (`self.Perform Stage Setup`))

(event `Perform Stage Setup`
  (bind _output_get (set `self.Current Stage` (+ (`self.Current Stage`) 1)))
  (`/Game/Widgets/WBP_HUD.Set New Level Title` (`self.HUD`) (`KismetStringLibrary.Concat_StrStr` "LEVEL " (`KismetStringLibrary.Conv_IntToString` _output_get)))
  (`KismetSystemLibrary.Delay` 4.0)
  (`/Game/Widgets/WBP_HUD.Hide Level Text` (`self.HUD`))
  (`self.Spawn New Stage`))

(event `Spawn New Stage`
  (bind _returnvalue (`|SpawnActorFromClass` "/Game/Blueprints/BP_Stage.BP_Stage_C" (`KismetMathLibrary.MakeTransform` (0.0 0.0 0.0)) "Undefined" "OverrideRootScale" null 2 false (`|MakeArray` (`self.GetTransform` (`self.Gate One`)) (`self.GetTransform` (`self.Gate Four`))) null))
  (bind _output_get (set `self.Active Stage` _returnvalue))
  (add `/Game/Blueprints/BP_Stage.Stage Completed` _output_get (delegate `Handle Stage Completed`))
  (`/Game/Blueprints/BP_Stage.Setup` (`self.Active Stage`)))

(event `Handle Stage Completed`)

(event `Restart`
  (bind _active_stage (`self.Active Stage`))
  ;[1 1 1] Restarts the current stage
  (`self.Reset Weapon Spawner`)
  (`/Engine/EditorBlueprintResources/StandardMacros.IsValid` _active_stage
    (:`Is Valid`
      (`/Game/Blueprints/BP_Stage.Teardown` _active_stage)
      (`/Game/Blueprints/BP_Stage.Setup` _active_stage))))

(event `Reset Weapon Spawner`
  (`/Engine/EditorBlueprintResources/StandardMacros.IsValid` (`self.Weapon Spawner`)
    (:`Is Valid`
      (`/Game/Blueprints/BP_WeaponAutoSpawner.Reset` (`self.Weapon Spawner`)))))

(fn `UserConstructionScript`)