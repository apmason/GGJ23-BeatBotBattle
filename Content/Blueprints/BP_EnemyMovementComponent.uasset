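; BP_EnemyMovementComponent is a component that walks its owning BP_Enemy in a straight line toward a given end location.
; StartWalking stores the speed and destination, caches the owner and its start location, and StopWalking clears the walking flag.
; While walking, Tick faces the enemy along the start-to-end direction and steps it forward at constant height, without delta-time scaling or an arrival check.
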(event `Start Walking`
  (params (Speed :type "Float (double-precision)") (`End Location` :type "Vector Structure"))
  (set `self.Can Walk` true)
  (set `self.Speed` Speed)
  (set `self.End Location` `End Location`)
  (bind _asbp_enemy (cast `/Game/Blueprints/BP_Enemy` (`self.GetOwner`))
    (:`then`
      (bind _output_get (set `self.Owning Enemy` _asbp_enemy))
      (set `self.Start Location` (`Actor.K2_GetActorLocation` _output_get)))
    (:`CastFailed`
      (`KismetSystemLibrary.PrintString` "EnemyMovementComponent doesn't have Enemy as owner!!" true true (struct :`R` 1.0 :`G` 0.022634 :`A` 1.0) 30.0))))

(event `self.ReceiveTick`
  (params (DeltaSeconds :type "Float (single-precision)"))
  (bind _owning_enemy (`self.Owning Enemy`))
  (bind _returnvalue (`Actor.K2_GetActorLocation` _owning_enemy))
  (bind (_returnvalue_x _returnvalue_y) (`KismetMathLibrary.BreakVector` (+ _returnvalue (* (`Actor.GetActorForwardVector` _owning_enemy) (`self.Speed`)))))
  (if (`self.Can Walk`)
    (`Actor.K2_SetActorRotation` (`self.Owning Enemy`) (`KismetMathLibrary.FindLookAtRotation` (`self.Start Location`) (`self.End Location`)) false)
    (`Actor.K2_SetActorLocation` (`self.Owning Enemy`) (`KismetMathLibrary.MakeVector` _returnvalue_x _returnvalue_y (.z _returnvalue)) false false)))

(event `Stop Walking`
  (set `self.Can Walk` false))